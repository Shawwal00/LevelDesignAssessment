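; EndingTrigger is a trigger Blueprint that sets off the ending sequence when any actor overlaps it.
; It destroys every actor tagged DeleteLight, and inside that same loop pauses the ClosedDoor's dust system and stops the RisingToxic's rise.
; Each iteration also sets an EndText flag and plays a camera shake at the player's location, so these effects depend on tagged actors existing.
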(event Collision|EventActorBeginOverlap
  (params (OtherActor :type Actor%20Object%20Reference))
  (bind _outactors (Actor|GetAllActorswithTag "DeleteLight"))
  (for _array_element _outactors
    (Actor|DestroyActor _array_element)
    (bind _returnvalue (Actor|GetActorOfClass "/Game/Blueprints/ClosedDoor.ClosedDoor_C"))
    (bind _asclosed_door (Utilities|Casting|CastToClosedDoor _returnvalue))
    (Class|NiagaraComponent|SetPaused (Variables|/Game/Blueprints/ClosedDoor.ClosedDoor_C|GetDust%20System _asclosed_door) true)
    (bind _returnvalue_2 (Actor|GetActorOfClass "/Game/Blueprints/Triggers/RisingToxic.RisingToxic_C"))
    (bind _asrising_toxic (Utilities|Casting|CastToRisingToxic _returnvalue_2))
    (Variables|/Game/Blueprints/Triggers/RisingToxic.RisingToxic_C|SetRise _asrising_toxic false)
    (Variables|Default|SetEndText true)
    (Camera|PlayWorldCameraShake "/Game/Blueprints/Camera.Camera_C" (Transformation|GetActorLocation (Game|GetPlayerCharacter 0)) 0.0 5e+02)))

(fn ConstructionScript)