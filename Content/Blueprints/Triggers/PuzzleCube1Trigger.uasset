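; One-shot puzzle trigger that repositions and reshapes the puzzle cubes when the player enters it.
; On overlap with the player character, it waits briefly, then gathers every PuzzleCubes actor in the level.
; Each cube drops along Z without sweeping, has its rotation zeroed and gets a fixed scale that is taller in Z.
; The trigger then destroys itself.
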(event Collision|EventActorBeginOverlap
  (params (OtherActor :type Actor%20Object%20Reference))
  (if (== OtherActor (Game|GetPlayerCharacter 0))
    (Utilities|FlowControl|Delay 1.0)
    (bind _outactors (Actor|GetAllActorsOfClass "/Game/Blueprints/Triggers/PuzzleCubes.PuzzleCubes_C"))
    (for _array_element _outactors
      (Transformation|SetActorTransform _array_element (Math|Transform|MakeTransform (- (Transformation|GetActorLocation _array_element) "0,0,100.000000") "0, 0, 0" "1.000000,1.000000,4.000000")))
    (Actor|DestroyActor)))

(fn ConstructionScript)