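; Trigger that makes a corridor appear to fall by rolling tagged pieces while the player overlaps it.
; Begin and end overlap with the player character toggle a Fall flag that gates Tick.
; Each frame it looks up every "Falling Slide" actor and uses RInterpTo toward an offset from its current roll, giving continuous rotation.
; The same loop fires a world camera shake at the player's location for each actor.
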(event Collision|EventActorBeginOverlap
  (params (OtherActor :type Actor%20Object%20Reference))
  (if (== OtherActor (Game|GetPlayerCharacter 0))
    (Variables|Default|SetFall true)))

(event EventTick
  (params (DeltaSeconds :type Float%20%28single-precision%29))
  (if (Variables|Default|GetFall)
    (bind _outactors (Actor|GetAllActorswithTag "Falling Slide"))
    (for _array_element _outactors
      (Transformation|SetActorRelativeRotation _array_element (Math|Interpolation|RInterpTo (Transformation|GetActorRotation _array_element) (Math|Rotator|MakeRotator (+ (.Roll (Math|Rotator|BreakRotator (Transformation|GetActorRotation _array_element))) 1e+02) (.Pitch (Math|Rotator|BreakRotator (Transformation|GetActorRotation _array_element))) (.Yaw (Math|Rotator|BreakRotator (Transformation|GetActorRotation _array_element)))) (Utilities|Time|GetWorldDeltaSeconds) 0.1))
      (Camera|PlayWorldCameraShake "/Game/Blueprints/FallingShake.FallingShake_C" (Transformation|GetActorLocation (Game|GetPlayerCharacter 0)) 0.0 5e+02))))

(event Collision|EventActorEndOverlap
  (params (OtherActor :type Actor%20Object%20Reference))
  (if (== OtherActor (Game|GetPlayerCharacter 0))
    (Variables|Default|SetFall false)))

(fn ConstructionScript)