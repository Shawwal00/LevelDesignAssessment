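; Third checkpoint trigger that updates the player's respawn point when the player character overlaps it.
; It writes its own location into RespawnLocation on BP_ThirdPersonCharacter.
; It then finds the ToxicPlane actor by class and moves it back to that plane's stored Start location.
; Nothing disables the trigger, so every new overlap repeats both steps.
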(event Collision|EventActorBeginOverlap
  (params (OtherActor :type Actor%20Object%20Reference))
  (if (== OtherActor (Game|GetPlayerCharacter 0))
    (bind _asbp_third_person_character (Utilities|Casting|CastToBP_ThirdPersonCharacter (Game|GetPlayerCharacter 0)))
    (Variables|/Game/ThirdPerson/Blueprints/BP_ThirdPersonCharacter.BP_ThirdPersonCharacter_C|SetRespawnLocation _asbp_third_person_character (Transformation|GetActorLocation))
    (bind _returnvalue (Actor|GetActorOfClass "/Game/Blueprints/ToxicPlane.ToxicPlane_C"))
    (bind _astoxic_plane (Utilities|Casting|CastToToxicPlane _returnvalue))
    (Transformation|SetActorLocation _astoxic_plane (Variables|/Game/Blueprints/ToxicPlane.ToxicPlane_C|GetStart _astoxic_plane) false false)))

(fn ConstructionScript)