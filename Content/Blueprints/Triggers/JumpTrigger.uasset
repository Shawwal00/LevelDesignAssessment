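; JumpTrigger is an interactable Blueprint that grants the player a triple jump.
; Interact casts player zero to BP_ThirdPersonCharacter, ignoring the interactor, raises its max jump count to three and sets the JumpText and Jump3 flags.
; Tick clears JumpText after a two-second delay, while Jump3 stays set.
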(event EventTick
  (params (DeltaSeconds :type Float%20%28single-precision%29))
  (if (Variables|Default|GetJumpText)
    (Utilities|FlowControl|Delay 2.0)
    (Variables|Default|SetJumpText false)))

(fn ConstructionScript)

(fn Interact
  (params (Interactor :type Character%20Object%20Reference))
  (bind _asbp_third_person_character (Utilities|Casting|CastToBP_ThirdPersonCharacter (Game|GetPlayerCharacter 0)))
  (Variables|/Script/Engine.Character|SetJumpMaxCount _asbp_third_person_character 3)
  (Variables|Default|SetJumpText true)
  (Variables|Default|SetJump3 true)
  (return true))