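; ClosedDoor is a door that cannot be moved by hand (Interact only prints a message) and opens once no PuzzleCube1Trigger remains in the level.
; Tick polls for that actor, and when none is found a timeline lerps the door's yaw open.
; A one-time guard spawns dust, swaps "DeleteWaste"-tagged meshes for toxic waste effects, shakes the camera and sets the player character's DoorOpen flag.
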(event EventTick
  (params (DeltaSeconds :type Float%20%28single-precision%29))
  (bind _returnvalue (Actor|GetActorOfClass "/Game/Blueprints/Triggers/PuzzleCube1Trigger.PuzzleCube1Trigger_C"))
  (Utilities|Casting|CastToPuzzleCube1Trigger _returnvalue
    (:CastFailed
      (bind _door_track (Timeline|Timeline_0 Play)
        (:Update
          (Transformation|SetRelativeRotation (Variables|Default|GetDoor) (Math|Rotator|MakeRotator 0.0 0.0 (Math|Float|Lerp (Variables|Default|GetClose%20Position) (Variables|Default|GetOpen%20Position) _door_track)) false false)
          (if (not (Variables|Default|GetOpen))
            (bind _returnvalue_2 (Niagara|SpawnSystematLocation "/Game/Niagras/DustSystem.DustSystem" "0,-4000.000000, 0"))
            (Variables|Default|SetOpen true)
            (Variables|Default|SetDust%20System _returnvalue_2)
            (bind _outactors (Actor|GetAllActorsOfClasswithTag "/Script/Engine.StaticMeshActor" "DeleteWaste"))
            (for _array_element _outactors
              (Niagara|SpawnSystematLocation "/Game/Niagras/ToxicWasteSystemGravity.ToxicWasteSystemGravity" (+ (Transformation|GetActorLocation _array_element) "-400.000000,60.000000,340.000000"))
              (Actor|DestroyActor _array_element)
              (Camera|PlayWorldCameraShake "/Game/Blueprints/Camera.Camera_C" (Transformation|GetActorLocation (Game|GetPlayerCharacter 0)) 0.0 5e+02)
              (bind _asbp_third_person_character (Utilities|Casting|CastToBP_ThirdPersonCharacter (Game|GetPlayerCharacter 0)))
              (Variables|/Game/ThirdPerson/Blueprints/BP_ThirdPersonCharacter.BP_ThirdPersonCharacter_C|SetDoorOpen _asbp_third_person_character true))))))))

(fn ConstructionScript)

(fn Interact
  (params (Interactor :type Character%20Object%20Reference))
  (Development|PrintText "This door cannot be moved")
  (return true))