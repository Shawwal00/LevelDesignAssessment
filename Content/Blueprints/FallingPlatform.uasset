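; A falling platform actor that drops after the player steps on it.
; Overlap with the player character waits through a short delay, then sets a Fall flag.
; While the flag is set, Tick moves the actor straight down by a fixed step each frame, without sweep or frame-time scaling, and nothing stops the descent.
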(event Collision|EventActorBeginOverlap
  (params (OtherActor :type Actor%20Object%20Reference))
  (if (== OtherActor (Game|GetPlayerCharacter 0))
    (Utilities|FlowControl|Delay 2.0)
    (Variables|Default|Setfall true)))

(event EventTick
  (params (DeltaSeconds :type Float%20%28single-precision%29))
  (if (Variables|Default|Getfall)
    (Transformation|SetActorLocation (+ (Transformation|GetActorLocation) "0,0,-10.000000") false false)))

(fn ConstructionScript)